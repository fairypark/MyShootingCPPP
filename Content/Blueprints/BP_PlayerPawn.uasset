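; Player pawn Blueprint for a shooting game, whose live graph only tracks health.
; BeginPlay sets Health to MaxHP, and OnMyUpdateHealth stores each new value it receives.
; Tick and the axis input events are empty.
; Unconnected leftover nodes hold movement, firing through components or direct BP_Bullet spawning with a blaster sound, and a game-over UI call to the game mode, none of which runs.
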(event `self.ReceiveBeginPlay`
  (set `self.health` (`self.maxHP`)))

(event `self.OnMyUpdateHealth`
  (params (value :type Integer))
  (set `self.health` value))

(event `self.ReceiveTick`
  (params (DeltaSeconds :type "Float (single-precision)"))
  ;[1 1 1] 사용자의 입력에따라 방향을 만들고
)

(event `InputAxis|Horizontal` :overrideparent false
  (params (AxisValue :type "Float (single-precision)")))

(event `InputAxis|Vertical` :overrideparent false
  (params (AxisValue :type "Float (single-precision)")))

(event `InputAction|Fire`
  (params (Key :type "Key Structure")))

(fn `UserConstructionScript`)
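; Game mode Blueprint for a shooting game, with a score counter and unwired game-over UI logic.
; AddScoreA adds the given value to the running score, and the SpawnDefaultPawnFor override returns without spawning a pawn.
; BeginPlay, Tick and ShowGameOverUI are empty.
; Disconnected nodes hold game-only input setup and a guarded creation of WBP_GameOver with animation, cursor and UI-only input.
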(event `self.ReceiveBeginPlay`)

(event `self.ReceiveTick`
  (params (DeltaSeconds :type "Float (single-precision)")))

(event `Event ShowGameOverUI`)

(fn `AddScoreA`
  (params (score :type Integer))
  (set `self.score_0` (+ score (`self.score_0`))))

(fn `SpawnDefaultPawnFor`
  (params (NewPlayer :type "Controller Object Reference") (StartSpot :type "Actor Object Reference"))
  (returns (ReturnValue :type "Pawn Object Reference"))
  (return null))

(fn `UserConstructionScript`)